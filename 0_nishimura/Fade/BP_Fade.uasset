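; BP_Fade is a screen-fade actor that creates a WBP_NormalFade widget on BeginPlay and adds it to the viewport.
; FadeInNormal and FadeOutNormal play its Fade animation forward or reversed, setting MIsFadeInNormal true on completion and false as soon as the reverse starts.
; Debug keys also drive normal and shutter fades with test prints, but the WBP_ShutterFade creation is unconnected, so that widget is never created here.
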(event Custom|FadeInNormal
  (bind _wbpnormalfade (Variables|Default|GetWBPNormalFade))
  (Components|Animation|PlayAnimation _wbpnormalfade (Variables|/Game/0_nishimura/Fade/WBP_NormalFade.WBP_NormalFade_C|GetFade _wbpnormalfade) 0.0
    (:Finished
      (Variables|Default|Setm_isFadeInNormal true))))

(event Custom|FadeOutNormal
  (bind _wbpnormalfade (Variables|Default|GetWBPNormalFade))
  (Components|Animation|PlayAnimation _wbpnormalfade (Variables|/Game/0_nishimura/Fade/WBP_NormalFade.WBP_NormalFade_C|GetFade _wbpnormalfade) 0.0 1 "Reverse"
    (:then
      (Variables|Default|Setm_isFadeInNormal false))))

(event EventBeginPlay
  (Input|EnableInput (Game|GetPlayerController 0))
  (bind _returnvalue (UserInterface|CreateWidget "/Game/0_nishimura/Fade/WBP_NormalFade.WBP_NormalFade_C"))
  (bind _output_get (Variables|Default|SetWBPNormalFade _returnvalue))
  (UserInterface|Viewport|AddtoViewport _output_get 0))

(event Input|KeyboardEvents|DebugKeyT
  (params (Key :type Key%20Structure :default "None") (ActionValue :type Input%20Action%20Value%20Structure))
  (bind _wbpnormalfade (Variables|Default|GetWBPNormalFade))
  (:Pressed
    (Components|Animation|PlayAnimation _wbpnormalfade (Variables|/Game/0_nishimura/Fade/WBP_NormalFade.WBP_NormalFade_C|GetFade _wbpnormalfade) 0.0 1 "Reverse"
      (:then
        (Development|PrintString "Hello"))
      (:Finished
        (Development|PrintString "endf")))))

(event Input|KeyboardEvents|DebugKeyH
  (params (Key :type Key%20Structure :default "None") (ActionValue :type Input%20Action%20Value%20Structure))
  (bind _wbpshutterfade (Variables|Default|GetWBPShutterFade))
  (:Pressed
    (Components|Animation|PlayAnimation _wbpshutterfade (Variables|/Game/0_nishimura/Fade/WBP_ShutterFade.WBP_ShutterFade_C|GetFade _wbpshutterfade) 0.0
      (:then
        (Development|PrintString "Hello"))
      (:Finished
        (Development|PrintString "endf")))))

(event Input|KeyboardEvents|DebugKeyJ
  (params (Key :type Key%20Structure :default "None") (ActionValue :type Input%20Action%20Value%20Structure))
  (bind _wbpshutterfade (Variables|Default|GetWBPShutterFade))
  (:Pressed
    (Components|Animation|PlayAnimation _wbpshutterfade (Variables|/Game/0_nishimura/Fade/WBP_ShutterFade.WBP_ShutterFade_C|GetFade _wbpshutterfade) 0.0 1 "Reverse"
      (:then
        (Development|PrintString "Hello"))
      (:Finished
        (Development|PrintString "endf")))))

(event Input|KeyboardEvents|SpaceBar
  (params (Key :type Key%20Structure :default "None"))
  (bind _wbpnormalfade (Variables|Default|GetWBPNormalFade))
  (:Pressed
    (Components|Animation|PlayAnimation _wbpnormalfade (Variables|/Game/0_nishimura/Fade/WBP_NormalFade.WBP_NormalFade_C|GetFade _wbpnormalfade) 0.0
      (:then
        (Development|PrintString "Hello"))
      (:Finished
        (Development|PrintString "endf")))))

(fn ConstructionScript)
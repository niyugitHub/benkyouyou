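; BP_Shatter is a breakable window actor that fades in its geometry collection, then triggers its destruction.
; While IsBreak is set, Tick calls FadeIn to step the Alpha parameter on two material slots, creating dynamic material instances on each call.
; Once the fade completes and a one-second delay passes, Break sets FieldActive on the BP_MasterField found in the level.
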(event `self.ReceiveTick`
  (params (DeltaSeconds :type "Float (single-precision)"))
  ;[1 1 1] 破壊可能になったら
  (if (`self.IsBreak`)
    ;[1 1 1] フェードイン処理をする
    (bind _isfadein (`self.FadeIn`))
    (set `self.IsPossibleBreak` _isfadein)
    (`KismetSystemLibrary.Delay` 1.0)
    ;[1 1 1] フェードイン処理が終わったら破壊する
    (if (`self.IsPossibleBreak`)
      (`self.Break`)
      (set `self.IsPossibleBreak` false))))

(fn `Break`
  (returns (`field Active` :type Boolean))
  (bind _returnvalue (`GameplayStatics.GetActorOfClass` "/Game/0_nishimura/RenderTarget/BP_MasterField.BP_MasterField_C"))
  (set `/Game/0_nishimura/RenderTarget/BP_MasterField.Field Active` true _returnvalue)
  (return true))

(fn `FadeIn`
  (returns (IsFadeIn :type Boolean))
  (bind _alphanum (`self.AlphaNum`))
  (bind _returnvalue (>= _alphanum 1.0))
  (set `self.AlphaNum` (+ (`self.AlphaNum`) 0.05))
  (bind _returnvalue_2 (`PrimitiveComponent.CreateDynamicMaterialInstance` (`self.SM_Window_1_GeometryCollection`) 0 null "None"))
  (bind _output_get (set `self.M_Alpha` _returnvalue_2))
  (`MaterialInstanceDynamic.SetScalarParameterValue` _output_get "Alpha" (`self.AlphaNum`))
  (bind _returnvalue_3 (`PrimitiveComponent.CreateDynamicMaterialInstance` (`self.SM_Window_1_GeometryCollection`) 1 null "None"))
  (bind _output_get_2 (set `self.M_Alpha` _returnvalue_3))
  (`MaterialInstanceDynamic.SetScalarParameterValue` _output_get_2 "Alpha" _alphanum)
  (if _returnvalue
    (set `self.AlphaNum` 1.0))
  (return _returnvalue))

(fn `UserConstructionScript`)
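; Player pawn for the end-roll credits that walks automatically along a fixed direction while the staff roll widget plays.
; Tick eases the spring arm's Y offset from its start position, then pins it at a stop position once the capsule nears it.
; Passing a skip point triggers a BP_Fade fade-in, then after a delay teleports the player's Y to the skip end and fades out.
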(event `self.ReceiveBeginPlay`
  ;[1 1 1] 始まった時にSpringArmのlocationをPlayerStartPos代入
  (set `self.m_cameraSpringArmStartPos` (.location (`SceneComponent.GetRelativeTransform` (`self.SpringArm`))))
  (bind _returnvalue (`|CreateWidget` "/Game/0_nishimura/Endroll/WBP_StaffRollText.WBP_StaffRollText_C"))
  (bind _output_get (set `self.m_wbpText` _returnvalue))
  (`UserWidget.AddToViewport` _output_get 0)
  (`/Game/0_nishimura/Endroll/WBP_StaffRollText.PlayStaffRoll` _output_get)
  (bind _returnvalue_2 (`GameplayStatics.GetActorOfClass` "/Game/0_nishimura/Fade/BP_Fade.BP_Fade_C"))
  (set `self.m_bpFade` _returnvalue_2))

(event `self.ReceiveTick`
  (params (DeltaSeconds :type "Float (single-precision)"))
  (bind _m_bpfade (`self.m_bpFade`))
  (if (> (`.Y` (`KismetMathLibrary.BreakVector3f` (`self.K2_GetActorLocation`))) (`.Y` (`KismetMathLibrary.BreakVector3f` (`self.m_skipPosStart`))))
    (if (not (`self.m_isSkip`))
      (set `self.m_isSkip` true)
      (`/Game/0_nishimura/Fade/BP_Fade.FadeInNormal` _m_bpfade)))
  (if (`/Game/0_nishimura/Fade/BP_Fade.m_isFadeInNormal` _m_bpfade)
    (`KismetSystemLibrary.Delay` 1.5)
    (`self.SkipPos`)
    (`/Game/0_nishimura/Fade/BP_Fade.FadeOutNormal` _m_bpfade))
  (`self.MovePlayer`) ; プレイヤーを移動させるための関数
  (set `self.m_time` (+ (/ DeltaSeconds 10.0) (`self.m_time`)))
  ;[1 1 1] 条件が合えばカメラを止める
  (bind _stopcamera (`self.IsStopCamera`))
  (if _stopcamera
    _
    (elif (`self.m_isMoveCamera`)
      ;[1 1 1] カメラを動かす処理
      (`self.Move Camera`))))

(fn `IsStopCamera`
  (returns (stopCamera :type Boolean))
  (bind _springarm (`self.SpringArm`))
  (bind (_x _y) (`KismetMathLibrary.BreakVector3f` (`self.m_stopCameraPos`)))
  (bind (_x_2 _y_2 _z) (`KismetMathLibrary.BreakVector3f` (`SceneComponent.K2_GetComponentLocation` _springarm)))
  (bind _returnvalue (> (`.Y` (`KismetMathLibrary.BreakVector3f` (`SceneComponent.K2_GetComponentLocation` (`self.CapsuleComponent`)))) (- _y 100.0)))
  (if _returnvalue
    (`SceneComponent.K2_SetWorldLocation` _springarm (`KismetMathLibrary.MakeVector` _x_2 _y _z) false false))
  (return _returnvalue))

(fn `Move Camera`
  (locals (NewLocalVar :type "Vector Structure" :default (0.0 0.0 0.0)))
  (set `self.m_cameraSpringArmPos` (`KismetMathLibrary.MakeVector` 0.0 (`|EaseFunction` "EaseOut" (`self.m_time`) (.y (`self.m_cameraSpringArmStartPos`)) 100.0)))
  (if (> (`self.m_time`) 1.0)
    (set `self.m_isMoveCamera` false)
    (set `self.m_cameraSpringArmPos` (0.0 100.0 0.0)))
  (`SceneComponent.K2_SetRelativeLocation` (`self.SpringArm`) (`self.m_cameraSpringArmPos`) false false)
  (return))

(fn `MovePlayer`
  (`self.AddMovementInput` (`self.m_playerVec`)))

(fn `SkipPos`
  (bind (_x _y _z) (`KismetMathLibrary.BreakVector3f` (`self.K2_GetActorLocation`)))
  (`self.K2_SetActorLocation` (`KismetMathLibrary.MakeVector` _x (`.Y` (`KismetMathLibrary.BreakVector3f` (`self.m_skipPosEnd`))) _z)))

(fn `UserConstructionScript`)
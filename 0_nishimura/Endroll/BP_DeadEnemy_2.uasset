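; Dead-enemy actor in the end-roll folder that plays a timed death effect on its skeletal mesh.
; Tick accumulates Time at one-fifth of real speed and passes it with the mesh to DeadEffect, which is defined outside this file.
; An unconnected branch would swap materials to M_Dead_Inst and call Dead, which writes Time to the "Qpaque" parameter on five dynamic material instances.
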(event `self.ReceiveBeginPlay`)

(event `self.ReceiveTick`
  (params (DeltaSeconds :type "Float (single-precision)"))
  (bind _time (`self.time`))
  (set `self.time` (+ (/ DeltaSeconds 5.0) _time))
  (`/Game/0_nishimura/FBP_Dead.DeadEffect` (`self.SkeletalMesh`) _time))

(fn `Dead`
  (bind _returnvalue (`PrimitiveComponent.CreateDynamicMaterialInstance` (`self.SkeletalMesh`) 0 null "None"))
  (`MaterialInstanceDynamic.SetScalarParameterValue` _returnvalue "Qpaque" (`self.time`))
  (bind _returnvalue_2 (`PrimitiveComponent.CreateDynamicMaterialInstance` (`self.SkeletalMesh`) 1 null "None"))
  (`MaterialInstanceDynamic.SetScalarParameterValue` _returnvalue_2 "Qpaque" (`self.time`))
  (bind _returnvalue_3 (`PrimitiveComponent.CreateDynamicMaterialInstance` (`self.SkeletalMesh`) 2 null "None"))
  (`MaterialInstanceDynamic.SetScalarParameterValue` _returnvalue_3 "Qpaque" (`self.time`))
  (bind _returnvalue_4 (`PrimitiveComponent.CreateDynamicMaterialInstance` (`self.SkeletalMesh`) 3 null "None"))
  (`MaterialInstanceDynamic.SetScalarParameterValue` _returnvalue_4 "Qpaque" (`self.time`))
  (bind _returnvalue_5 (`PrimitiveComponent.CreateDynamicMaterialInstance` (`self.SkeletalMesh`) 4 null "None"))
  (`MaterialInstanceDynamic.SetScalarParameterValue` _returnvalue_5 "Qpaque" (`self.time`)))

(fn `UserConstructionScript`)
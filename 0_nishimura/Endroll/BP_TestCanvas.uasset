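; BP_TestCanvas is a test Blueprint for showing the end-roll staff credits through WidgetBackGround and WidgetText components.
; BeginPlay and the construction script are empty, so none of its logic runs.
; Disconnected nodes would enable player input, create viewport copies of both components' widget classes, and call PlayStaffRoll on the text widget.
; The stored widget variables are set to None rather than the created widgets.
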(event EventBeginPlay)

(event Input|KeyboardEvents|DebugKeyT
  (params (Key :type Key%20Structure :default "None") (ActionValue :type Input%20Action%20Value%20Structure)))

(fn ConstructionScript)